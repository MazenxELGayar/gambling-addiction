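; Player-controlled flying drone pawn that fires blaster beams.
; Enhanced Input drives floating movement on all three axes relative to control rotation and controller look, with the mesh snapped to control rotation every tick.
; Firing alternates between right and left rifle sockets via a FlipFlop, spawning a beam actor, burst effect and sound.
; A toggle switches between single shots and auto fire, which is rate-limited by a flag and Delay.
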(event Input|EnhancedActionEvents|EnhancedInputActionIA_PawnBotFire
  (params (ActionValue :type Boolean) (ElapsedSeconds :type Float%20%28double-precision%29) (TriggeredSeconds :type Float%20%28double-precision%29) (InputAction :type Input%20Action%20Object%20Reference :default "/Game/Input/Actions/Drone/IA_PawnBotFire.IA_PawnBotFire"))
  ;[200 0 0 0.071] Blasting
  (:Triggered
    (if (Variables|Default|GetBlastingAuto)
      (if (not (Variables|Default|GetBlastingStarted))
        (Variables|Default|SetBlastingStarted true)
        (bind _isa (Utilities|FlowControl|FlipFlop :!label _label)
          (:A
            _)
          (:B
            _))
        (CallFunction|SpawnBlasterBeams _isa)
        (Utilities|FlowControl|Delay (Variables|Default|GetBlastingRate))
        (Variables|Default|SetBlastingStarted false))))
  (:Started
    (if (not (Variables|Default|GetBlastingAuto))
      (goto _label))))

(event Input|EnhancedActionEvents|EnhancedInputActionIA_PawnBotToggleAuto
  (params (ActionValue :type Boolean) (ElapsedSeconds :type Float%20%28double-precision%29) (TriggeredSeconds :type Float%20%28double-precision%29) (InputAction :type Input%20Action%20Object%20Reference :default "/Game/Input/Actions/Drone/IA_PawnBotToggleAuto.IA_PawnBotToggleAuto"))
  ;[0.02144 0.3698 0.1536] Toggle Auto
  (:Completed
    (CallFunction|ToggleAuto)))

(event Input|EnhancedActionEvents|EnhancedInputActionIA_PawnBotLook
  (params (ActionValue :type Vector%202D%20Structure) (ElapsedSeconds :type Float%20%28double-precision%29) (TriggeredSeconds :type Float%20%28double-precision%29) (InputAction :type Input%20Action%20Object%20Reference :default "/Game/Input/Actions/Drone/IA_PawnBotLook.IA_PawnBotLook"))
  ;[0.02144 0.3698 0.1536] Look Around
  (CallFunction|LookAround ActionValue))

(event Input|EnhancedActionEvents|EnhancedInputActionIA_PawnBotMove
  (params (ActionValue :type Vector :default "0, 0, 0") (ElapsedSeconds :type Float%20%28double-precision%29) (TriggeredSeconds :type Float%20%28double-precision%29) (InputAction :type Input%20Action%20Object%20Reference :default "/Game/Input/Actions/Drone/IA_PawnBotMove.IA_PawnBotMove"))
  ;[0.02144 0.3698 0.1536] Move
  (CallFunction|Move ActionValue))

(event EventBeginPlay
  ;[0.02144 0.3698 0.1536] Start Mapping
  (CallFunction|AddBotInputMapping))

(event EventTick
  (params (DeltaSeconds :type Float%20%28single-precision%29))
  ;[0.02144 0.3698 0.1536] Rotate Drone With Cam
  (CallFunction|RotateDronewithCamera))

(fn ConstructionScript)

(fn AddBotInputMapping
  (bind _asplayer_controller (Utilities|Casting|CastToPlayerController (Pawn|GetController)))
  (Input|AddMappingContext (PlayerController|LocalPlayerSubsystems|GetEnhancedInputLocalPlayerSubsystem _asplayer_controller) "/Game/Input/IMC_PawnBot.IMC_PawnBot" 0 "(bIgnoreAllPressedKeysUntilRelease=True,bForceImmediately=False,bNotifyUserSettings=False)"))

(fn InitializeSocketVariables
  (Utilities|FlowControl|Sequence))

(fn SpawnBlasterBeams
  (params (isRightBeam :type Boolean))
  (bind _botmesh (Variables|Default|GetBotMesh))
  (bind _botmesh_2 (Variables|Default|GetBotMesh))
  (bind _riffle_l_socket_name (Variables|Components|GetRiffle_L_Socket_Name))
  (bind _riffle_r_socket_name (Variables|Components|GetRiffle_R_Socket_Name))
  (bind _returnvalue (Transformation|GetSocketTransform _botmesh _riffle_r_socket_name "RTS_World"))
  (bind _returnvalue_2 (Transformation|GetSocketTransform _botmesh_2 _riffle_l_socket_name "RTS_World"))
  (bind _returnvalue_3 (select isRightBeam _returnvalue _returnvalue_2))
  (bind (_location _rotation) (Math|Transform|BreakTransform _returnvalue_3))
  (Game|SpawnActorfromClass "/Game/BluePrints/Drone/BP_BlasterBeam.BP_BlasterBeam_C" _returnvalue_3 "Undefined" "MultiplyWithRoot" 0 0 (Variables|Components|GetBlaster%20Beam%20Damage_0) 0 0)
  (Niagara|SpawnSystematLocation "/Game/Assets/FX/NS_BeamBurst.NS_BeamBurst" _location _rotation)
  (Audio|PlaySoundatLocation "/Game/Assets/Sounds/Drone/SFX_EngeryRifle.SFX_EngeryRifle" "0, 0, 0" "0, 0, 0" 1.0 1.0 0.0 0 0 0 0)
  (return _returnvalue_3))

(fn ToggleAuto
  (Variables|Default|SetBlastingAuto (not (Variables|Default|GetBlastingAuto))))

(fn LookAround
  (params (InVec :type Vector%202D%20Structure))
  (bind (_x _y) (Math|Vector2D|BreakVector2D InVec))
  (Utilities|FlowControl|Sequence
    (:then_0
      (Pawn|Input|AddControllerYawInput _x))
    (:then_1
      (Pawn|Input|AddControllerPitchInput _y))))

(fn RotateDronewithCamera
  (Transformation|SetWorldRotation (Variables|Default|GetBotMesh) (Pawn|GetControlRotation :!class /Script/Engine.Pawn) false false))

(fn Move
  (params (InVec :type Vector))
  (bind (_x _y _z) (Math|Vector|BreakVector InVec))
  (Utilities|FlowControl|Sequence
    (:then_0
      (CallFunction|MoveLeftRight _x))
    (:then_1
      (CallFunction|MoveForwardBackward _y))
    (:then_2
      (CallFunction|MoveUpDown _z))))

(fn MoveForwardBackward
  (params (Y :type Float%20%28double-precision%29))
  (Class|PawnMovementComponent|AddInputVector (Variables|Default|GetFloatingPawnMovement) (* Y (Math|Vector|GetForwardVector (Pawn|GetControlRotation :!class /Script/Engine.Pawn))) false))

(fn MoveLeftRight
  (params (X :type Float%20%28double-precision%29))
  (Class|PawnMovementComponent|AddInputVector (Variables|Default|GetFloatingPawnMovement) (* X (Math|Vector|GetRightVector (Pawn|GetControlRotation :!class /Script/Engine.Pawn))) false))

(fn MoveUpDown
  (params (Z :type Float%20%28double-precision%29))
  (Class|PawnMovementComponent|AddInputVector (Variables|Default|GetFloatingPawnMovement) (* Z (Math|Vector|GetUpVector (Pawn|GetControlRotation :!class /Script/Engine.Pawn))) false))