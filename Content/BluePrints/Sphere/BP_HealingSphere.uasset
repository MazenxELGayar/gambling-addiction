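; BP_HealingSphere is an actor pickup that heals a BP_ThirdPersonCharacter that hits it.
; It binds OnActorHit on BeginPlay, then destroys itself and adds HealingAmount to the character's HP on a matching hit.
; PrintNewHp shows the healing on screen in green, though its total adds HealingAmount again to the already updated HP.
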(event Custom|OnActorHit_Event
  (params (SelfActor :type Actor%20Object%20Reference) (OtherActor :type Actor%20Object%20Reference) (NormalImpulse :type Vector) (Hit :type Hit%20Result%20Structure%20%28by%20ref%29))
  (bind _asbp_third_person_character (Utilities|Casting|CastToBP_ThirdPersonCharacter OtherActor))
  (bind _fullhealth (CallFunction|DestroyBallandHealPlayer _asbp_third_person_character))
  (CallFunction|PrintNewHp _asbp_third_person_character _fullhealth))

(event EventBeginPlay
  (Collision|AssignOnActorHit (delegate Custom|OnActorHit_Event)))

(fn ConstructionScript)

(fn PrintNewHp
  (params (Pawn :type BP%20Third%20Person%20Character%20Object%20Reference) (FullHealth :type Integer))
  (Development|PrintString (Utilities|String|Append (Utilities|GetDisplayName Pawn) " +" (Utilities|String|ToString(Integer) (Variables|Default|GetHealingAmount)) " , FullHp: " (Utilities|String|ToString(Integer) FullHealth)) true true "(R=0.021441,G=0.369792,B=0.153612,A=1.000000)" 5.0))

(fn DestroyBallandHealPlayer
  (params (Player :type BP%20Third%20Person%20Character%20Object%20Reference))
  (Actor|DestroyActor)
  (Variables|/Game/ThirdPerson/Blueprints/BP_ThirdPersonCharacter.BP_ThirdPersonCharacter_C|SetHP Player (+ (Variables|/Game/ThirdPerson/Blueprints/BP_ThirdPersonCharacter.BP_ThirdPersonCharacter_C|GetHP Player) (Variables|Default|GetHealingAmount)))
  (return (+ (Variables|/Game/ThirdPerson/Blueprints/BP_ThirdPersonCharacter.BP_ThirdPersonCharacter_C|GetHP Player) (Variables|Default|GetHealingAmount))))