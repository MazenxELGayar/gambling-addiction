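; Play-as-bot game-mode Blueprint handling events that spawn or kill allies and enemies, or heal the instigator.
; Ally/enemy roles are mostly inverted: ally events use BP_Bot (or human characters via EnemiesAreBots), enemy events BP_PawnBot, though DestroyAlly also targets BP_PawnBot.
; DestroyorSpawn events roll configurable odds to spawn or kill.
; Spawns use random reachable points around the instigator; kills fall back to random actors and credit the instigator.
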(event EventDestroyAlly
  (params (SpecificAlly :type Actor%20Object%20Reference) (InestigatorActor :type Actor%20Object%20Reference))
  ;[0.008758 0.151 0.06274] DestroyOrSpawnEnemy
  (Destroy|DestroySpecificorRandomAllyBot SpecificAlly InestigatorActor))

(event EventSpawnAlly
  (params (InestigatorActor :type Actor%20Object%20Reference))
  ;[0.008758 0.151 0.06274] DestroyOrSpawnEnemy
  (Spawning|SpawnEnemyBot InestigatorActor))

(event EventDestroyEnemy
  (params (SpecificEnemy :type Actor%20Object%20Reference) (InestigatorActor :type Actor%20Object%20Reference))
  ;[0.008758 0.151 0.06274] DestroyOrSpawnEnemy
  (Destroy|DestroySpecificorRandomAllyBot SpecificEnemy InestigatorActor))

(event EventSpawnEnemy
  (params (InestigatorActor :type Actor%20Object%20Reference))
  ;[0.008758 0.151 0.06274] DestroyOrSpawnEnemy
  (Spawning|SpawnAllyPawn InestigatorActor))

(event EventDestroyorSpawnAlly
  (params (DestroySpecificAlly :type Actor%20Object%20Reference) (InestigatorActor :type Actor%20Object%20Reference))
  ;[0.008758 0.151 0.06274] DestroyOrSpawnEnemy
  (CallFunction|DestroyorSpawnEnemyFunction DestroySpecificAlly InestigatorActor))

(event EventDestroyorSpawnEnemy
  (params (DestroySpecificEnemy :type Actor%20Object%20Reference) (InestigatorActor :type Actor%20Object%20Reference))
  ;[0.008758 0.151 0.06274] DestroyOrSpawnEnemy
  (CallFunction|DestroyorSpawnAllyFunction DestroySpecificEnemy InestigatorActor))

(event EventHealPlayer
  (params (InestigatorActor :type Actor%20Object%20Reference))
  ;[0.008758 0.151 0.06274] HealPlayer
  (bind _asbpi_get_hurt (Utilities|Casting|CastToBPI_GetHurt InestigatorActor))
  (Default|Heal _asbpi_get_hurt (Variables|Default|GetHealAmount) InestigatorActor))

(fn ConstructionScript)

(fn SpawnEnemyHuman
  (params (InestigatorActor :type Actor%20Object%20Reference))
  (Game|SpawnActorfromClass "/Game/BluePrints/Human/BP_ThirdPersonCharacter.BP_ThirdPersonCharacter_C" (Location|GetSpawnLocation InestigatorActor) "Undefined" "MultiplyWithRoot" InestigatorActor 0))

(fn SpawnEnemyBot
  (params (InestigatorActor :type Actor%20Object%20Reference))
  (Game|SpawnActorfromClass "/Game/BluePrints/Drone/BP_Bot.BP_Bot_C" (Location|GetSpawnLocation InestigatorActor) "Undefined" "MultiplyWithRoot" InestigatorActor 0))

(fn SpawnAllyPawn
  (params (InestigatorActor :type Actor%20Object%20Reference))
  (bind _returnvalue (Game|SpawnActorfromClass "/Game/BluePrints/Drone/BP_PawnBot.BP_PawnBot_C" (Location|GetSpawnLocation InestigatorActor) "Undefined" "MultiplyWithRoot" 0 0))
  (Development|PrintString (Utilities|String|Append (Utilities|GetDisplayName InestigatorActor) " spawned " (Utilities|GetDisplayName _returnvalue))))

(fn DestroySpecificorRandomEnemyBot
  (params (SpeceficEnemy :type Object%20Object%20Reference) (InestigatorActor :type Actor%20Object%20Reference))
  (bind _asbp_bot (Utilities|Casting|CastToBP_Bot SpeceficEnemy)
    (:then
      (Default|DieInstantly _asbp_bot (Transformation|GetActorTransform _asbp_bot) InestigatorActor))
    (:CastFailed
      (bind _outactors (Actor|GetAllActorsOfClass "/Game/BluePrints/Drone/BP_Bot.BP_Bot_C"))
      (Utilities|IsValid (.OutItem (Utilities|Array|Random _outactors))
        (:Is%20Valid
          (Class|BPIGetHurt|DieInstantly(Message) (.OutItem (Utilities|Array|Random _outactors)) (Transformation|GetActorTransform (.OutItem (Utilities|Array|Random _outactors))) InestigatorActor)))))
  (Utilities|IsValid InestigatorActor
    (:Is%20Valid
      (Class|BPIGetHurt|IncreaseKilledAllies(Message) InestigatorActor 1))))

(fn DestroySpecificorRandomHuman
  (params (SpeceficEnemy :type Object%20Object%20Reference) (InestigatorActor :type Actor%20Object%20Reference))
  (bind _asbp_third_person_character (Utilities|Casting|CastToBP_ThirdPersonCharacter SpeceficEnemy)
    (:then
      (Default|DieInstantly _asbp_third_person_character (Transformation|GetActorTransform _asbp_third_person_character) InestigatorActor))
    (:CastFailed
      (bind _outactors (Actor|GetAllActorsOfClass "/Game/BluePrints/Human/BP_ThirdPersonCharacter.BP_ThirdPersonCharacter_C"))
      (Utilities|IsValid (.OutItem (Utilities|Array|Random _outactors))
        (:Is%20Valid
          (Class|BPIGetHurt|DieInstantly(Message) (.OutItem (Utilities|Array|Random _outactors)) (Transformation|GetActorTransform (.OutItem (Utilities|Array|Random _outactors))) InestigatorActor)))))
  (Utilities|IsValid InestigatorActor
    (:Is%20Valid
      (Class|BPIGetHurt|IncreaseKilledAllies(Message) InestigatorActor 1))))

(fn DestroySpecificorRandomAllyBot
  (params (SpeceficBot :type Object%20Object%20Reference) (InestigatorActor :type Actor%20Object%20Reference))
  (bind _asbp_pawn_bot (Utilities|Casting|CastToBP_PawnBot SpeceficBot)
    (:then
      (Default|DieInstantly _asbp_pawn_bot (Transformation|GetActorTransform _asbp_pawn_bot) InestigatorActor))
    (:CastFailed
      (bind _outactors (Actor|GetAllActorsOfClass "/Game/BluePrints/Drone/BP_PawnBot.BP_PawnBot_C"))
      (Utilities|IsValid (.OutItem (Utilities|Array|Random _outactors))
        (:Is%20Valid
          (Default|DieInstantly (.OutItem (Utilities|Array|Random _outactors)) (Transformation|GetActorTransform (.OutItem (Utilities|Array|Random _outactors))) InestigatorActor)))))
  (Utilities|IsValid InestigatorActor
    (:Is%20Valid
      (Class|BPIGetHurt|IncreaseKilledEnimies(Message) InestigatorActor 1))))

(fn GetSpawnLocation
  (params (Inestigator :type Actor%20Object%20Reference))
  (bind _output_get (LocalVariables|SetInestigatorArg Inestigator))
  (Utilities|IsValid _output_get
    (:Is%20Valid
      (LocalVariables|SetSpawnTransform (Location|GetRandomSpawnLocationfromPlayer (LocalVariables|GetInestigatorArg))))
    (:Is%20Not%20Valid
      (bind _outactors (Actor|GetAllActorsOfClass "/Game/BluePrints/Human/BP_ThirdPersonCharacter.BP_ThirdPersonCharacter_C"))
      (Utilities|IsValid (.OutItem (Utilities|Array|Random _outactors))
        (:Is%20Valid
          (LocalVariables|SetSpawnTransform (Location|GetRandomSpawnLocationfromPlayer (.OutItem (Utilities|Array|Random _outactors))))))))
  (return (LocalVariables|GetSpawnTransform)))

(fn GetRandomSpawnLocationfromPlayer
  (params (Inestigator :type Actor%20Object%20Reference))
  (return (Math|Conversions|ToTransform(Vector) (+ (.RandomLocation (AI|Navigation|GetRandomReachablePointinRadius (Transformation|GetActorLocation Inestigator) (Math|Random|RandomFloatinRange (Variables|Default|GetMinSphereSpawningRadius) (Variables|Default|GetMaxSphereSpawningRadius)) 0 0)) "0.000000,0.000000,100.000000"))))

(fn DestroyorSpawnAllyFunction
  (params (SpeceficBot :type Object%20Object%20Reference) (InestigatorActor :type Actor%20Object%20Reference))
  ;[0.008758 0.151 0.06274] DestroyOrSpawnAlly
  (if (<= (Math|Random|RandomFloatinRange 0.0 1.0) (Variables|Default|GetCreate%20Ally%20Instead%20Of%20Destroy%20Percentage))
    (Spawning|SpawnAllyPawn InestigatorActor)
    (else
      (Destroy|DestroySpecificorRandomAllyBot SpeceficBot InestigatorActor))))

(fn DestroyorSpawnEnemyFunction
  (params (SpecficEnemy :type Actor%20Object%20Reference) (Inestigator :type Actor%20Object%20Reference))
  (Utilities|FlowControl|Sequence
    (:then_0
      (LocalVariables|SetSpecficEnemyArg SpecficEnemy))
    (:then_1
      (LocalVariables|SetInestigatorArg Inestigator))
    (:then_2
      (if (<= (Math|Random|RandomFloatinRange 0.0 1.0) (Variables|Default|GetCreate%20Enemy%20Instead%20Of%20Destroy%20Percentage))
        (if (Variables|Default|GetEnemiesAreBots?)
          (Spawning|SpawnEnemyBot (LocalVariables|GetInestigatorArg))
          (else
            (Spawning|SpawnEnemyHuman (LocalVariables|GetInestigatorArg))))
        (elif (Variables|Default|GetEnemiesAreBots?)
          (Destroy|DestroySpecificorRandomEnemyBot (LocalVariables|GetSpecficEnemyArg) (LocalVariables|GetInestigatorArg))
          (else
            (Destroy|DestroySpecificorRandomHuman (LocalVariables|GetSpecficEnemyArg) (LocalVariables|GetInestigatorArg))))))))