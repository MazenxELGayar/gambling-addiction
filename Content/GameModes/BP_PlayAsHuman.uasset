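; BP_PlayAsHuman is the play-as-human game mode logic, where allies are third-person human characters and enemies are bots.
; Its events spawn, destroy or heal characters, with combined events rolling a chance to spawn instead of destroy.
; Spawns use random navmesh-reachable points around the instigator or a fallback random human.
; Destruction kills the specified target or a random one of that class and increments the instigator's kill count.
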(event EventDestroyAlly
  (params (SpecificAlly :type Actor%20Object%20Reference) (InestigatorActor :type Actor%20Object%20Reference))
  ;[0.008758 0.151 0.06274] DestroyOrSpawnAlly
  (CallFunction|DestroySpecificorRandomAlly SpecificAlly InestigatorActor))

(event EventSpawnAlly
  (params (InestigatorActor :type Actor%20Object%20Reference))
  ;[0.008758 0.151 0.06274] DestroyOrSpawnAlly
  (CallFunction|SpawnAllyHuman InestigatorActor))

(event EventDestroyEnemy
  (params (SpecificEnemy :type Actor%20Object%20Reference) (InestigatorActor :type Actor%20Object%20Reference))
  ;[0.008758 0.151 0.06274] DestroyOrSpawnEnemy
  (CallFunction|DestroySpecificorRandomBot SpecificEnemy InestigatorActor))

(event EventSpawnEnemy
  (params (InestigatorActor :type Actor%20Object%20Reference))
  ;[0.008758 0.151 0.06274] DestroyOrSpawnEnemy
  (CallFunction|SpawnEnemyBot InestigatorActor))

(event EventDestroyorSpawnAlly
  (params (DestroySpecificAlly :type Actor%20Object%20Reference) (InestigatorActor :type Actor%20Object%20Reference))
  ;[0.008758 0.151 0.06274] DestroyOrSpawnAlly
  (if (<= (Math|Random|RandomFloatinRange 0.0 1.0) (Variables|Default|GetCreate%20Ally%20Instead%20Of%20Destroy%20Percentage))
    (CallFunction|SpawnAllyHuman InestigatorActor)
    (else
      (CallFunction|DestroySpecificorRandomAlly DestroySpecificAlly InestigatorActor))))

(event EventDestroyorSpawnEnemy
  (params (DestroySpecificEnemy :type Actor%20Object%20Reference) (InestigatorActor :type Actor%20Object%20Reference))
  ;[0.008758 0.151 0.06274] DestroyOrSpawnEnemy
  (if (<= (Math|Random|RandomFloatinRange 0.0 1.0) (Variables|Default|GetCreate%20Enemy%20Instead%20Of%20Destroy%20Percentage))
    (CallFunction|SpawnEnemyBot InestigatorActor)
    (else
      (CallFunction|DestroySpecificorRandomBot DestroySpecificEnemy InestigatorActor))))

(event EventHealPlayer
  (params (InestigatorActor :type Actor%20Object%20Reference))
  ;[0.008758 0.151 0.06274] HealPlayer
  (bind _asbp_third_person_character (Utilities|Casting|CastToBP_ThirdPersonCharacter InestigatorActor))
  (Default|Heal _asbp_third_person_character (Variables|Default|GetHealAmount)))

(fn ConstructionScript)

(fn SpawnEnemyBot
  (params (InestigatorActor :type Actor%20Object%20Reference))
  (Game|SpawnActorfromClass "/Game/BluePrints/Drone/BP_Bot.BP_Bot_C" (CallFunction|GetSpawnLocation InestigatorActor) "Undefined" "MultiplyWithRoot" 0 0))

(fn SpawnAllyHuman
  (params (InestigatorActor :type Actor%20Object%20Reference))
  (bind _returnvalue (Game|SpawnActorfromClass "/Game/BluePrints/Human/BP_ThirdPersonCharacter.BP_ThirdPersonCharacter_C" (CallFunction|GetSpawnLocation InestigatorActor) "AdjustIfPossibleButAlwaysSpawn" "MultiplyWithRoot" 0 0))
  (Development|PrintString (Utilities|String|Append (Utilities|GetDisplayName InestigatorActor) " spawned " (Utilities|GetDisplayName _returnvalue)))
  (Default|MovetoClosestSphere _returnvalue))

(fn DestroySpecificorRandomBot
  (params (SpeceficBot :type Object%20Object%20Reference) (InestigatorActor :type Actor%20Object%20Reference))
  (bind _asbp_bot (Utilities|Casting|CastToBP_Bot SpeceficBot)
    (:then
      (Default|DieInstantly _asbp_bot (Transformation|GetActorTransform _asbp_bot)))
    (:CastFailed
      (bind _outactors (Actor|GetAllActorsOfClass "/Game/BluePrints/Drone/BP_Bot.BP_Bot_C"))
      (Utilities|IsValid (.OutItem (Utilities|Array|Random _outactors))
        (:Is%20Valid
          (Default|DieInstantly (.OutItem (Utilities|Array|Random _outactors)) (Transformation|GetActorTransform (.OutItem (Utilities|Array|Random _outactors))))))))
  (Utilities|IsValid InestigatorActor
    (:Is%20Valid
      (Class|BPIGetHurt|IncreaseKilledEnimies(Message) InestigatorActor 1))))

(fn DestroySpecificorRandomAlly
  (params (SpeceficAlly :type Object%20Object%20Reference) (InestigatorActor :type Actor%20Object%20Reference))
  (bind _asbp_third_person_character (Utilities|Casting|CastToBP_ThirdPersonCharacter SpeceficAlly)
    (:then
      (Default|DieInstantly _asbp_third_person_character (Transformation|GetActorTransform _asbp_third_person_character) InestigatorActor))
    (:CastFailed
      (bind _outactors (Actor|GetAllActorsOfClass "/Game/BluePrints/Human/BP_ThirdPersonCharacter.BP_ThirdPersonCharacter_C"))
      (Utilities|IsValid (.OutItem (Utilities|Array|Random _outactors))
        (:Is%20Valid
          (Class|BPIGetHurt|DieInstantly(Message) (.OutItem (Utilities|Array|Random _outactors)) (Transformation|GetActorTransform (.OutItem (Utilities|Array|Random _outactors))) InestigatorActor)))))
  (Utilities|IsValid InestigatorActor
    (:Is%20Valid
      (Class|BPIGetHurt|IncreaseKilledAllies(Message) InestigatorActor 1))))

(fn GetSpawnLocation
  (params (Inestigator :type Actor%20Object%20Reference))
  (bind _output_get (LocalVariables|SetInestigatorArg Inestigator))
  (Utilities|IsValid _output_get
    (:Is%20Valid
      (LocalVariables|SetSpawnTransform (CallFunction|GetRandomSpawnLocationfromPlayer (LocalVariables|GetInestigatorArg))))
    (:Is%20Not%20Valid
      (bind _outactors (Actor|GetAllActorsOfClass "/Game/BluePrints/Human/BP_ThirdPersonCharacter.BP_ThirdPersonCharacter_C"))
      (Utilities|IsValid (.OutItem (Utilities|Array|Random _outactors))
        (:Is%20Valid
          (LocalVariables|SetSpawnTransform (CallFunction|GetRandomSpawnLocationfromPlayer (.OutItem (Utilities|Array|Random _outactors))))))))
  (return (LocalVariables|GetSpawnTransform)))

(fn GetRandomSpawnLocationfromPlayer
  (params (Inestigator :type Actor%20Object%20Reference))
  (return (Math|Conversions|ToTransform(Vector) (+ (.RandomLocation (AI|Navigation|GetRandomReachablePointinRadius (Transformation|GetActorLocation Inestigator) (Math|Random|RandomFloatinRange (Variables|Default|GetMinSphereSpawningRadius) (Variables|Default|GetMaxSphereSpawningRadius)) 0 0)) "0.000000,0.000000,100.000000"))))

(fn ProjectileMovementVelocity
  (return (Variables|Default|GetBlasterBeamSpeed)))